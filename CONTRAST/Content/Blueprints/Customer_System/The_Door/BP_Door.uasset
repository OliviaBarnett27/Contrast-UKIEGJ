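; BP_Door is a shop door that swings open for customers and plays a bell sound.
; A BP_Customer overlapping the Outside trigger plays a timeline that rotates the door, with DoOnce gates limiting the opening and bell.
; Two seconds after the bell, it enables the Box trigger, whose customer overlap reverses the timeline to close the door.
; Four seconds later, it disables Box and resets both gates.
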(event OnComponentBeginOverlap(Outside)
  (params (OverlappedComponent :type Primitive%20Component%20Object%20Reference) (OtherActor :type Actor%20Object%20Reference) (OtherComp :type Primitive%20Component%20Object%20Reference) (OtherBodyIndex :type Integer) (bFromSweep :type Boolean) (SweepResult :type Hit%20Result%20Structure%20%28by%20ref%29))
  (Utilities|Casting|CastToBP_Customer OtherActor)
  (Utilities|FlowControl|DoOnce false
    (:Completed
      (bind _dooropen (Timeline|DoorOpen PlayFromStart)
        (:Update
          (Transformation|SetRelativeRotation (Variables|Default|GetDoor_BECC17E8) (Math|Rotator|Lerp(Rotator) "0, 0, 0" "0.000000,120.000000,0.000000" _dooropen) false false)
          (Utilities|FlowControl|DoOnce false
            (:Completed
              (Audio|SpawnSoundatLocation "/Game/audio/door_bell/556710__nachtmahrtv__shop-bell.556710__nachtmahrtv__shop-bell" (Transformation|GetWorldLocation (Variables|Default|GetDoor_BECC17E8)) "0, 0, 0" 1.0 1.0 0.0 0 0)
              (Utilities|FlowControl|Delay 2.0)
              (Collision|SetCollisionEnabled (Variables|Default|GetBox) "QueryOnly"))))))))

(event OnComponentBeginOverlap(Box)
  (params (OverlappedComponent :type Primitive%20Component%20Object%20Reference) (OtherActor :type Actor%20Object%20Reference) (OtherComp :type Primitive%20Component%20Object%20Reference) (OtherBodyIndex :type Integer) (bFromSweep :type Boolean) (SweepResult :type Hit%20Result%20Structure%20%28by%20ref%29))
  (Utilities|Casting|CastToBP_Customer OtherActor)
  (Utilities|FlowControl|Sequence
    (:then_0
      (Utilities|FlowControl|Delay 4.0)
      (Collision|SetCollisionEnabled (Variables|Default|GetBox) "NoCollision")
      (Utilities|FlowControl|Sequence
        (:then_0
          (Utilities|FlowControl|DoOnce false) ; enters at Reset
        )
        (:then_1
          (goto _label Reset))))
    (:then_1
      (bind _dooropen (Timeline|DoorOpen Reverse)
        (:Update
          (Transformation|SetRelativeRotation (Variables|Default|GetDoor_BECC17E8) (Math|Rotator|Lerp(Rotator) "0, 0, 0" "0.000000,120.000000,0.000000" _dooropen) false false)
          (Utilities|FlowControl|DoOnce false :!label _label
            (:Completed
              (Audio|SpawnSoundatLocation "/Game/audio/door_bell/556710__nachtmahrtv__shop-bell.556710__nachtmahrtv__shop-bell" (Transformation|GetWorldLocation (Variables|Default|GetDoor_BECC17E8)) "0, 0, 0" 1.0 1.0 0.0 0 0)
              (Utilities|FlowControl|Delay 2.0)
              (Collision|SetCollisionEnabled (Variables|Default|GetBox) "QueryOnly"))))))))

(event EventBeginPlay
  (Collision|SetCollisionEnabled (Variables|Default|GetBox) "NoCollision"))

(fn ConstructionScript)