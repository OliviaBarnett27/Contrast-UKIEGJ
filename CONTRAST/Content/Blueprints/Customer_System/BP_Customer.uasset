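; BP_Customer is a customer that picks one of three random shape orders, walks to a counter and later leaves.
; Chained AIMoveTo calls follow hard-coded waypoints, departing after a short wait or once served.
; An OrderBox overlap destroys any BP_OrderItem, and AcceptOrder checks its type, showing the held mesh and setting a flag.
; Tick polls that flag through DoOnce to leave, fire completion and item-used calls, then destroy the actor.
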(event OnComponentBeginOverlap(OrderBox)
  (params (OverlappedComponent :type Primitive%20Component%20Object%20Reference) (OtherActor :type Actor%20Object%20Reference) (OtherComp :type Primitive%20Component%20Object%20Reference) (OtherBodyIndex :type Integer) (bFromSweep :type Boolean) (SweepResult :type Hit%20Result%20Structure%20%28by%20ref%29))
  (bind _asbp_order_item (Utilities|Casting|CastToBP_OrderItem OtherActor))
  (CallFunction|AcceptOrder (Variables|/Game/Blueprints/Orders/BP_OrderItem.BP_OrderItem_C|GetOrderType _asbp_order_item))
  (Actor|DestroyActor _asbp_order_item))

(event Custom|MoveToCounter
  (AI|AIMoveTo self "2050.000000,1100.000000,110.000000" 0 5.0 false
    (:OnSuccess
      (AI|AIMoveTo self "1270.000000,1100.000000,110.000000" 0 5.0 false
        (:OnSuccess
          (Utilities|FlowControl|Delay 5.0)
          (CallFunction|LeaveCounter)
          (Default|CallOnOrderComplete)
          (Utilities|FlowControl|Delay 7.0)
          (Actor|DestroyActor))))))

(event Custom|LeaveCounter
  (AI|AIMoveTo self "2050.000000,1100.000000,110.000000" 0 5.0 false
    (:OnSuccess
      (AI|AIMoveTo self "2050.000000,360.000000,110.000000" 0 5.0 false))))

(event EventBeginPlay
  (CallFunction|AssignOrder)
  (CallFunction|MovetoCounter))

(event EventTick
  (params (DeltaSeconds :type Float%20%28single-precision%29))
  (if (Variables|Default|GetHasRecievedOrder)
    (Utilities|FlowControl|DoOnce false
      (:Completed
        (CallFunction|LeaveCounter)
        (Default|CallOnOrderComplete)
        (Utilities|FlowControl|Delay 7.0)
        (Default|CallOnItemUsed)
        (Actor|DestroyActor)))))

(fn ConstructionScript)

(fn AssignOrder
  (Variables|Default|SetOrderType (Utilities|Enum|ByteToEnumEnum_OrderType (Math|Conversions|ToByte(Integer) (Math|Random|RandomIntegerinRange 0 2)))))

(fn AcceptOrder
  (params (OrderType :type Enum_OrderType%20Enum :default "NewEnumerator0"))
  (bind _orderitemheld (Variables|Default|GetOrderItemHeld))
  (if (Utilities|Enum|Equal(Enum) OrderType (Variables|Default|GetOrderType))
    (Variables|Default|SetHasRecievedOrder true)
    (switch Utilities|FlowControl|Switch|SwitchonEnum_OrderType (Variables|Default|GetOrderType)
      (:NewEnumerator0
        (Components|StaticMesh|SetStaticMesh _orderitemheld "/Engine/BasicShapes/Sphere.Sphere"))
      (:NewEnumerator1
        (Components|StaticMesh|SetStaticMesh _orderitemheld "/Game/StarterContent/Shapes/Shape_Cube.Shape_Cube"))
      (:NewEnumerator2
        (Components|StaticMesh|SetStaticMesh _orderitemheld "/Game/StarterContent/Shapes/Shape_Cylinder.Shape_Cylinder")))))