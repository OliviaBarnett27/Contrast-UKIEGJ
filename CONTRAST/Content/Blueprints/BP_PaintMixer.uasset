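; BP_PaintMixer is a clickable paint mixer actor that opens colour selection for the player.
; It binds its click event on BeginPlay; a click prints and then clears the player pawn's holding-can message flag.
; The click also blends the camera view to the mixer and adds a new WBP_ColourSelection widget to the viewport.
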(event Custom|OnClicked_Event
  (params (TouchedActor :type Actor%20Object%20Reference) (ButtonPressed :type Key%20Structure :default "None"))
  (bind _returnvalue (Game|Player|GetPlayerPawn 0))
  (bind _isholdingcan (Class|BPIPaintCan|GetHoldingCan(Message) _returnvalue))
  (Development|PrintString (Utilities|String|Append "holding can: " (Utilities|String|ToString(Boolean) _isholdingcan)))
  (Class|BPIPaintCan|SetHoldingCan(Message) _returnvalue false)
  (Game|Player|SetViewTargetwithBlend (Game|GetPlayerController 0) self 0.0 "VTBlend_Linear" 0.0 false)
  (bind _returnvalue_2 (UserInterface|CreateWidget "/Game/CONTRAST/UI/WBP_ColourSelection.WBP_ColourSelection_C"))
  (UserInterface|Viewport|AddtoViewport _returnvalue_2 0))

(event EventBeginPlay
  (EventDispatchers|AssignOnClicked (delegate Custom|OnClicked_Event)))

(fn ConstructionScript)