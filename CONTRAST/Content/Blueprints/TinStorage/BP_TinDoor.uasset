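; BP_TinDoor is a sliding door for the tin storage that raises its mesh upward and triggers delivery of a tin.
; OpenDoors plays a timeline that lerps the Cube's relative position, and closedoor reverses it from the end.
; A DoOnce on timeline updates plays the hatch sound and, if the player holds no can, calls BP_Tin's BringForthTin.
; The DoOnce resets only on that delivery path, after a short delay.
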(event Custom|Open%20Doors
  (bind _opening (Timeline|DoorMoving PlayFromStart)
    (:Update
      (Transformation|SetRelativeLocation (Variables|Default|GetCube) (Math|Vector|Lerp(Vector) "0, 0, 0" "0.000000,0.000000,90.000000" _opening) false false)
      (Utilities|FlowControl|DoOnce false :!label _label
        (:Completed
          (Audio|SpawnSoundatLocation "/Game/audio/metal_door/446108__justinvoke__hatchdoor-open.446108__justinvoke__hatchdoor-open" (Transformation|GetWorldLocation (Variables|Default|GetCube)) "0, 0, 0" 1.0 1.0 0.0 0 0)
          (bind _returnvalue (Actor|GetActorOfClass "/Game/ThirdPerson/Blueprints/BP_ThirdPersonCharacter.BP_ThirdPersonCharacter_C"))
          (if (not (Variables|/Game/ThirdPerson/Blueprints/BP_ThirdPersonCharacter.BP_ThirdPersonCharacter_C|GetIs%20Holding%20Can _returnvalue))
            (bind _returnvalue_2 (Actor|GetActorOfClass "/Game/Blueprints/TinStorage/BP_Tin.BP_Tin_C"))
            (Default|BringForthTin _returnvalue_2)
            (Utilities|FlowControl|Delay 2.0)
            (goto _label Reset)))))))

(event Custom|close%20door
  (bind _opening (Timeline|DoorMoving ReverseFromEnd)
    (:Update
      (Transformation|SetRelativeLocation (Variables|Default|GetCube) (Math|Vector|Lerp(Vector) "0, 0, 0" "0.000000,0.000000,90.000000" _opening) false false)
      (Utilities|FlowControl|DoOnce false :!label _label
        (:Completed
          (Audio|SpawnSoundatLocation "/Game/audio/metal_door/446108__justinvoke__hatchdoor-open.446108__justinvoke__hatchdoor-open" (Transformation|GetWorldLocation (Variables|Default|GetCube)) "0, 0, 0" 1.0 1.0 0.0 0 0)
          (bind _returnvalue (Actor|GetActorOfClass "/Game/ThirdPerson/Blueprints/BP_ThirdPersonCharacter.BP_ThirdPersonCharacter_C"))
          (if (not (Variables|/Game/ThirdPerson/Blueprints/BP_ThirdPersonCharacter.BP_ThirdPersonCharacter_C|GetIs%20Holding%20Can _returnvalue))
            (bind _returnvalue_2 (Actor|GetActorOfClass "/Game/Blueprints/TinStorage/BP_Tin.BP_Tin_C"))
            (Default|BringForthTin _returnvalue_2)
            (Utilities|FlowControl|Delay 2.0)
            (goto _label Reset)))))))

(fn ConstructionScript)