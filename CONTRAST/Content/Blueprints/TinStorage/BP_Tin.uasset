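; BP_Tin is a tin that a crane claw delivers and the player picks up.
; BringForthTin runs timelines that lower the tin and claw, then slide the tin sideways with a conveyor sound played once while the claw rises again.
; Interact tells the third-person character to grab the can, moves the tin to a fixed world position, and resets the door, red button lever and sound gate.
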(event Custom|BringForthTin
  (bind _tin (Variables|Default|GetTin))
  (Utilities|FlowControl|Sequence
    (:then_0
      (bind _tindown (Timeline|TinDown PlayFromStart)
        (:Update
          (Transformation|SetRelativeLocation _tin (Math|Vector|Lerp(Vector) "0, 0, 0" "0.000000,0.000000,-153.000000" _tindown) false false))
        (:Finished
          (Utilities|FlowControl|Delay 1.0)
          (bind _tindown_2 (Timeline|TinAcross PlayFromStart)
            (:Update
              (Utilities|FlowControl|Sequence
                (:then_0
                  (Transformation|SetRelativeLocation _tin (Math|Vector|Lerp(Vector) "0.000000,0.000000,-153.000000" "0.000000,280.000000,-153.000000" _tindown_2) false false))
                (:then_1
                  (Utilities|FlowControl|DoOnce false
                    (:Completed
                      (bind _returnvalue (Audio|SpawnSoundatLocation "/Game/audio/conveyer/83226__smokum__convey-1.83226__smokum__convey-1" (Transformation|GetWorldLocation (Variables|Default|GetTin)) "0, 0, 0" 1.0 1.0 0.0 0 0)))))))
            (:Finished
              (Audio|Components|Audio|Stop _returnvalue))))))
    (:then_1
      (bind _tindown_3 (Timeline|Timeline PlayFromStart)
        (:Update
          (Transformation|SetRelativeLocation (Variables|Default|GetCrane_and_Lever_Crane_Claw) (Math|Vector|Lerp(Vector) "0, 0, 0" "0.000000,0.000000,-140.000000" _tindown_3) false false))
        (:Finished
          (Utilities|FlowControl|Delay 2.0)
          (bind _tindown_4 (Timeline|Timeline_0 Play)
            (:Update
              (Transformation|SetRelativeLocation (Variables|Default|GetCrane_and_Lever_Crane_Claw) (Math|Vector|Lerp(Vector) "0.000000,0.000000,-140.000000" "0.000000,0.000000,140.000000" _tindown_4) false false))))))))

(event EventInteract
  (Utilities|FlowControl|Sequence
    (:then_0
      (bind _returnvalue (Actor|GetActorOfClass "/Game/ThirdPerson/Blueprints/BP_ThirdPersonCharacter.BP_ThirdPersonCharacter_C"))
      (Default|GrabsCan _returnvalue)
      (Transformation|SetWorldLocation (Variables|Default|GetTin) "917.000000,380.000000,400.000000" false false))
    (:then_1
      (bind _returnvalue_2 (Actor|GetActorOfClass "/Game/Blueprints/TinStorage/BP_TinDoor.BP_TinDoor_C"))
      (Default|CloseDoor _returnvalue_2))
    (:then_2
      (bind _returnvalue_3 (Actor|GetActorOfClass "/Game/Blueprints/TinStorage/BP_RedButton.BP_RedButton_C"))
      (Default|LeverDownReset _returnvalue_3))
    (:then_3
      (Utilities|FlowControl|DoOnce false) ; enters at Reset
    )
    (:then_4
      (Audio|SpawnSound2D "/Game/audio/interact/665181__el_boss__item-or-material-pickup-pop-3-of-3.665181__el_boss__item-or-material-pickup-pop-3-of-3" 1.0 1.0 0.0 0))))

(fn ConstructionScript)