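; BP_Customer is an AI paintbrush customer that requests a random paint colour at the counter.
; It picks a brush mesh and blinking face, walks in via AIMoveTo, shows its widget and waits on a timed delay.
; Interact compares the player's can colour to the order, updating the player's correct or incorrect tally through message calls.
; A timeout or Tick-detected correct order makes it leave, signal completion and destroy itself.
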(event Custom|MoveToCounter
  (AI|AIMoveTo self "2050.000000,1100.000000,110.000000" 0 5.0 false
    (:OnSuccess
      (AI|AIMoveTo self "1200.000000,1100.000000,110.000000" 0 5.0 false
        (:OnSuccess
          (Rendering|SetVisibility (Variables|Default|GetWidget) true false)
          (Utilities|FlowControl|Delay 2e+01)
          (CallFunction|LeaveCounter)
          (Default|CallOnOrderComplete)
          (Utilities|FlowControl|Delay 7.0)
          (Actor|DestroyActor))))))

(event Custom|LeaveCounter
  (Rendering|SetVisibility (Variables|Default|GetWidget) true false)
  (AI|AIMoveTo self "2050.000000,1100.000000,110.000000" 0 5.0 false
    (:OnSuccess
      (AI|AIMoveTo self "2050.000000,360.000000,110.000000" 0 5.0 false))))

(event EventBeginPlay
  (CallFunction|AssignModel)
  (CallFunction|AssignOrder)
  (CallFunction|MovetoCounter))

(event EventInteract
  (bind _returnvalue (Game|Player|GetPlayerPawn 0))
  (bind _isholdingcan (Class|BPIPaintCan|GetHoldingCan(Message) _returnvalue))
  (if _isholdingcan
    (bind _paintenum (Class|BPIPaintCan|GetCanPaintColour(Message) _returnvalue))
    (CallFunction|AcceptOrder _paintenum)))

(event EventTick
  (params (DeltaSeconds :type Float%20%28single-precision%29))
  (if (Variables|Default|GetHasRecievedOrder)
    (Utilities|FlowControl|DoOnce false
      (:Completed
        (CallFunction|LeaveCounter)
        (Default|CallOnOrderComplete)
        (Utilities|FlowControl|Delay 7.0)
        (Default|CallOnItemUsed)
        (Actor|DestroyActor)))))

(fn ConstructionScript)

(fn AssignOrder
  (Variables|Default|SetOrderType (Utilities|Enum|ByteToEnumEnum_OrderType (Math|Conversions|ToByte(Integer) (Math|Random|RandomIntegerinRange 0 5)))))

(fn AcceptOrder
  (params (PlayerOrderType :type Enum_OrderType%20Enum :default "NewEnumerator6"))
  (bind _returnvalue (Game|Player|GetPlayerPawn 0))
  (bind _returnvalue_2 (Game|Player|GetPlayerPawn 0))
  (if (Utilities|Enum|Equal(Enum) PlayerOrderType (Variables|Default|GetOrderType))
    ;[0.403 1 0.5311] Correct
    (Variables|Default|SetHasRecievedOrder true)
    (Audio|SpawnSound2D "/Game/audio/interact/665181__el_boss__item-or-material-pickup-pop-3-of-3.665181__el_boss__item-or-material-pickup-pop-3-of-3" 1.0 1.0 0.0 0)
    (bind _returnvalue_3 (Actor|GetActorOfClass "/Game/ThirdPerson/Blueprints/BP_ThirdPersonCharacter.BP_ThirdPersonCharacter_C"))
    (Variables|/Game/ThirdPerson/Blueprints/BP_ThirdPersonCharacter.BP_ThirdPersonCharacter_C|SetIs%20Holding%20Can _returnvalue_3 false)
    (Rendering|SetVisibility (Variables|/Game/ThirdPerson/Blueprints/BP_ThirdPersonCharacter.BP_ThirdPersonCharacter_C|GetPaintTin _returnvalue_3) false false)
    (bind _orderscompleted (Class|BPIPlayerInformation|GetOrdersCompleted(Message) _returnvalue_2))
    (Class|BPIPlayerInformation|SetOrdersCompleted(Message) _returnvalue_2 (+ _orderscompleted 1))
    (else
      (bind _ordersincorrect (Class|BPIPlayerInformation|GetOrdersIncorrect(Message) _returnvalue))
      (bind _result (Math|Integer|IncrementInt _ordersincorrect)
        (:%20%20
          (Class|BPIPlayerInformation|SetOrdersIncorrect(Message) _returnvalue _result))))))

(fn AssignModel
  (bind _brushesarray (Variables|Default|GetBrushesArray))
  (bind _keys (Utilities|Map|Keys _brushesarray))
  (bind _output_get (Variables|Default|SetNewVar (.OutItem (Utilities|Array|Random _keys))))
  (Components|StaticMesh|SetStaticMesh (Variables|Default|GetBrushModel) (.OutItem (Utilities|Array|Random _keys)))
  (Variables|Default|SetAngle%20Face (.IdleFace (Utilities|Struct|BreakStruct_Face (.Value (Utilities|Map|Find _brushesarray _output_get)))))
  (Variables|Default|SetAngle%20Face%20Blink (.FaceBlink (Utilities|Struct|BreakStruct_Face (.Value (Utilities|Map|Find _brushesarray _output_get)))))
  (Utilities|Time|SetTimerbyFunctionName 0 "Face" 1.0 true))

(fn Face
  (bind _brushface (Variables|Default|GetBrushFace))
  (if (== (Variables|Default|GetFaceNumber) 1)
    (Rendering|Material|SetMaterial _brushface 0 (Variables|Default|GetAngle%20Face))
    (Variables|Default|SetFaceNumber (- (Variables|Default|GetFaceNumber) 1))
    (else
      (Rendering|Material|SetMaterial _brushface 0 (Variables|Default|GetAngle%20Face%20Blink))
      (Variables|Default|SetFaceNumber (+ (Variables|Default|GetFaceNumber) 1)))))