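; BP_CustomerSpawner spawns BP_Customer actors at a fixed hardcoded transform, tracking the latest one as CurrentCustomer.
; BeginPlay spawns the first customer and binds HandleOrderComplete to its OnOrderComplete event, which spawns another after a short delay.
; SpawnCustomer also binds a delegate to each new customer's OnOrderComplete.
; Despite its name, SpawnNextCustomer only repeats the BeginPlay binding on CurrentCustomer, without spawning.
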(event Custom|Spawn%20Next%20Customer
  (EventDispatchers|BindEventtoOnOrderComplete (Variables|Default|GetCurrentCustomer) (delegate Custom|HandleOrderComplete)))

(event Custom|HandleOrderComplete
  (Utilities|FlowControl|Delay 7.0)
  (CallFunction|SpawnCustomer))

(event EventBeginPlay
  (CallFunction|SpawnCustomer)
  (EventDispatchers|BindEventtoOnOrderComplete (Variables|Default|GetCurrentCustomer) (delegate Custom|HandleOrderComplete)))

(fn ConstructionScript)

(fn SpawnCustomer
  (bind _returnvalue (Game|SpawnActorfromClass "/Game/Blueprints/Customer_System/BP_Customer.BP_Customer_C" (Math|Transform|MakeTransform "2050.000000,1850.000000,110.000000" "0.000000,-90.000000,0.000000" "1.000000,1.000000,1.000000") "Undefined" "MultiplyWithRoot" 0 0))
  (bind _output_get (Variables|Default|SetCurrentCustomer _returnvalue))
  (EventDispatchers|BindEventtoOnOrderComplete _output_get (EventDispatchers|CreateEvent :!event Custom|HandleOrderComplete)))